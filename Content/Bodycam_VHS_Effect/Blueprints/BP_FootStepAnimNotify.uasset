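; Anim notify that plays a footstep sound when an animation reaches it.
; It line traces 200 units down from the owning actor on the Visibility channel and, on a hit, reads the surface type.
; The surface switch has no distinct per-surface sounds, only a single carpet footstep cue.
; The cue's location is set to the world origin rather than the actor or hit point.
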(fn ReceivedNotify
  (params (MeshComp :type Skeletal%20Mesh%20Component%20Object%20Reference) (Animation :type Anim%20Sequence%20Base%20Object%20Reference) (EventReference :type Anim%20Notify%20Event%20Reference%20Structure%20%28by%20ref%29))
  (bind _returnvalue (Components|GetOwner MeshComp))
  (bind _returnvalue_2 (Transformation|GetActorLocation _returnvalue))
  (bind (_outhit _returnvalue_3) (Collision|LineTraceByChannel _returnvalue_2 (+ _returnvalue_2 (* (Transformation|GetActorUpVector _returnvalue) -2e+02)) "TraceTypeQuery1" false 0 "None" true "(R=1.000000,G=0.000000,B=0.000000,A=1.000000)" "(R=0.000000,G=1.000000,B=0.000000,A=1.000000)" 3.0))
  (if _returnvalue_3
    (switch Utilities|FlowControl|Switch|SwitchonEPhysicalSurface (Collision|GetSurfaceType _outhit)
      (:SurfaceType_Default
        (Audio|PlaySoundatLocation "/Game/Bodycam_VHS_Effect/Sounds/FootSteps/S_FootStep_Carpet_Cue.S_FootStep_Carpet_Cue" "0, 0, 0" "0, 0, 0" 1.0 1.0 0.0 0 0 0 0))))
  (return false))